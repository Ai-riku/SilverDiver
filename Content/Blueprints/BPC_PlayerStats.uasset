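; Actor component that tracks the player's health, stamina, XP and level on the third-person character.
; Increase and decrease functions adjust each stat; decreases return true once health or stamina is depleted.
; XP overflow carries into IncreaseLevel, which raises the XP threshold by the new level and recurses for multi-level gains.
; Stat changes push values straight into the owning character's HUD widget bars and texts.
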(event `self.ReceiveBeginPlay`
  (bind _asbp_third_person_character (cast `/Game/ThirdPerson/Blueprints/BP_ThirdPersonCharacter` (`self.GetOwner`)))
  (set `self.Player Character BP` _asbp_third_person_character))

(fn `Decrease Health`
  (params (`Health Decrease` :type "Float (double-precision)"))
  (returns (`Is Player Dead?` :type Boolean))
  (if (not (<= (`self.Current Health`) 0.0))
    (set `self.Current Health` (- (`self.Current Health`) `Health Decrease`))
    (`self.Update Health HUD`)
    (if (<= (`self.Current Health`) 0.0)
      (set `self.Current Health` 0.0)
      (else
        (return false))))
  (return true))

(fn `Decrease Stamina`
  (params (`Stamina Decrease` :type "Float (double-precision)"))
  (returns (`Stamina Depleted` :type Boolean))
  (if (not (<= (`self.Current Stamina`) 0.0))
    (set `self.Current Stamina` (- (`self.Current Stamina`) `Stamina Decrease`))
    (`self.Update Stamina HUD`)
    (if (<= (`self.Current Stamina`) 0.0)
      (set `self.Current Stamina` 0.0)
      (else
        (return false))))
  (return true))

(fn `Increase Health`
  (params (`Health Increase` :type "Float (double-precision)"))
  (bind _max_health (`self.Max Health`))
  (set `self.Current Health` (+ (`self.Current Health`) `Health Increase`))
  (if (> (`self.Current Health`) _max_health)
    (set `self.Current Health` _max_health))
  (`self.Update Health HUD`))

(fn `Increase Level`
  (params (`Level Increase` :type Integer))
  (set `self.Level` (+ (`self.Level`) `Level Increase`))
  (set `self.Max XP` (+ (`self.Max XP`) (* (`self.Level`) 50)))
  (`self.Update Level and XP HUD`)
  (if (>= (`self.XP`) (`self.Max XP`))
    (set `self.XP` (- (`self.XP`) (`self.Max XP`)))
    (`self.Increase Level` 1)))

(fn `Increase Max Health`
  (params (`Max Health Increase` :type "Float (double-precision)"))
  (set `self.Max Health` (+ (`self.Max Health`) `Max Health Increase`))
  (`self.Update Health HUD`))

(fn `Increase Max Stamina`
  (params (`Max Stamina Increase` :type "Float (double-precision)"))
  (set `self.Max Stamina` (+ (`self.Max Stamina`) `Max Stamina Increase`))
  (`self.Update Stamina HUD`))

(fn `Increase Stamina`
  (params (`Stamina Increase` :type "Float (double-precision)"))
  (bind _max_stamina (`self.Max Stamina`))
  (set `self.Current Stamina` (+ (`self.Current Stamina`) `Stamina Increase`))
  (if (> (`self.Current Stamina`) _max_stamina)
    (set `self.Current Stamina` _max_stamina))
  (`self.Update Stamina HUD`))

(fn `Increase XP`
  (params (`XP Increase` :type "Float (double-precision)"))
  (set `self.XP` (+ (`self.XP`) `XP Increase`))
  (`self.Update Level and XP HUD`)
  (if (>= (`self.XP`) (`self.Max XP`))
    (set `self.XP` (- (`self.XP`) (`self.Max XP`)))
    (`self.Increase Level` 1)))

(fn `Update Health HUD`
  (bind _current_health (`self.Current Health`))
  (bind _max_health (`self.Max Health`))
  (bind _hud_widget (`/Game/ThirdPerson/Blueprints/BP_ThirdPersonCharacter.HUD Widget` (`self.Player Character BP`)))
  (`ProgressBar.SetPercent` (`/Game/UI/WB_HUD.HealthBar` _hud_widget) (/ _current_health _max_health))
  (`TextBlock.SetText` (`/Game/UI/WB_HUD.HealthText` _hud_widget) (`KismetTextLibrary.Conv_StringToText` (`KismetStringLibrary.Concat_StrStr` (`KismetStringLibrary.Concat_StrStr` (`KismetStringLibrary.Conv_DoubleToString` _current_health) "/") (`KismetStringLibrary.Conv_DoubleToString` _max_health)))))

(fn `Update HUD`
  (`self.Update Health HUD`)
  (`self.Update Stamina HUD`)
  (`self.Update Level and XP HUD`))

(fn `Update Level and XP HUD`
  (bind _xp (`self.XP`))
  (bind _max_xp (`self.Max XP`))
  (bind _hud_widget (`/Game/ThirdPerson/Blueprints/BP_ThirdPersonCharacter.HUD Widget` (`self.Player Character BP`)))
  (`ProgressBar.SetPercent` (`/Game/UI/WB_HUD.XPBar` _hud_widget) (/ _xp _max_xp))
  (`TextBlock.SetText` (`/Game/UI/WB_HUD.XPText` _hud_widget) (`KismetTextLibrary.Conv_StringToText` (`KismetStringLibrary.Concat_StrStr` (`KismetStringLibrary.Concat_StrStr` (`KismetStringLibrary.Conv_DoubleToString` _xp) "/") (`KismetStringLibrary.Conv_DoubleToString` _max_xp))))
  (`TextBlock.SetText` (`/Game/UI/WB_HUD.LevelText` _hud_widget) (`KismetTextLibrary.Conv_IntToText` (`self.Level`))))

(fn `Update Stamina HUD`
  (`ProgressBar.SetPercent` (`/Game/UI/WB_HUD.StaminaBar` (`/Game/ThirdPerson/Blueprints/BP_ThirdPersonCharacter.HUD Widget` (`self.Player Character BP`))) (/ (`self.Current Stamina`) (`self.Max Stamina`))))