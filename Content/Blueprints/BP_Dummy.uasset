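; BP_Dummy is a target character that takes damage, can be stealth-assassinated from behind, and ragdolls on death.
; Damage plays a random hit montage and sound, launches it along the player's facing, and updates a camera-facing health bar that hides after a retriggerable delay.
; An overlap radius toggles the assassinate prompt for the player.
; StealthBackAssassin plays the victim montage, returns the attacker's alignment transform, and triggers delayed death.
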(event `self.ReceiveTick`
  (params (DeltaSeconds :type "Float (single-precision)"))
  (bind _heath_bar_widget (`self.Heath Bar Widget`))
  (`SceneComponent.K2_SetWorldRotation` _heath_bar_widget (`KismetMathLibrary.FindLookAtRotation` (`SceneComponent.K2_GetComponentLocation` _heath_bar_widget) (`SceneComponent.K2_GetComponentLocation` (`PlayerCameraManager.TransformComponent` (`GameplayStatics.GetPlayerCameraManager` 0)))) false false))

(event `self.ReceiveBeginPlay`
  (bind _aswb_dummy_health_bar (cast `/Game/UI/WB_DummyHealthBar` (`WidgetComponent.GetWidget` (`self.Heath Bar Widget`))))
  (set `self.Health Bar Widget` _aswb_dummy_health_bar)
  (`self.Update HUD`))

(event `self.Assassination Radius.OnComponentBeginOverlap`
  (params (OverlappedComponent :type "PrimitiveComponent Object Reference") (OtherActor :type "Actor Object Reference") (OtherComp :type "PrimitiveComponent Object Reference") (OtherBodyIndex :type Integer) (bFromSweep :type Boolean) (SweepResult :type "HitResult Structure (by ref)"))
  (cast `/Game/ThirdPerson/Blueprints/BP_ThirdPersonCharacter` OtherActor)
  (`SceneComponent.SetVisibility` (`self.Assassinate Widget`) true false))

(event `self.Assassination Radius.OnComponentEndOverlap`
  (params (OverlappedComponent :type "PrimitiveComponent Object Reference") (OtherActor :type "Actor Object Reference") (OtherComp :type "PrimitiveComponent Object Reference") (OtherBodyIndex :type Integer))
  (cast `/Game/ThirdPerson/Blueprints/BP_ThirdPersonCharacter` OtherActor)
  (`SceneComponent.SetVisibility` (`self.Assassinate Widget`) false false))

(event `self.ReceiveAnyDamage`
  (params (Damage :type "Float (single-precision)") (DamageType :type "DamageType Object Reference") (InstigatedBy :type "Controller Object Reference") (DamageCauser :type "Actor Object Reference"))
  (bind _returnvalue (`self.K2_GetActorLocation`))
  (bind _hit_animations (`self.Hit Animations`))
  ;[0.05127 0.05127 0.05127] Damage
  (`self.PlayAnimMontage` (`|GetArrayItem` _hit_animations (`KismetMathLibrary.RandomIntegerInRange` 0 (`KismetArrayLibrary.Array_Length` _hit_animations))))
  (bind _asbp_third_person_character (cast `/Game/ThirdPerson/Blueprints/BP_ThirdPersonCharacter` (`GameplayStatics.GetPlayerCharacter` 0)))
  (`self.LaunchCharacter` (* (`KismetMathLibrary.GetForwardVector` (`self.K2_GetActorRotation` _asbp_third_person_character)) 700.0))
  (bind _is_player_dead_ (`/Game/Blueprints/BPC_Character_Stats.Decrease Health` (`self.BPC_Character_Stats`) Damage))
  (`self.Update Health HUD`)
  (`self.Unhide Health Bar`)
  (if _is_player_dead_
    (`GameplayStatics.PlaySoundAtLocation` "/Game/Audio/Grunts-Hits/SC_Death.SC_Death" _returnvalue (struct) 1.0 1.0 0.0 null null null null)
    (`self.Die`)
    (else
      (`GameplayStatics.PlaySoundAtLocation` "/Game/Audio/Grunts-Hits/Death1.Death1" _returnvalue (struct) 1.0 (`KismetMathLibrary.RandomFloatInRange` 0.8 1.2) 0.0 null null null null))))

(event `Unhide Health Bar`
  (bind _heath_bar_widget (`self.Heath Bar Widget`))
  ;[0.05127 0.05127 0.05127] Damage
  (`SceneComponent.SetVisibility` _heath_bar_widget true false)
  (`KismetSystemLibrary.RetriggerableDelay` 5.0)
  (`SceneComponent.SetVisibility` _heath_bar_widget false false))

(event `Die`
  (bind _mesh (`self.Mesh`))
  ;[0.05127 0.05127 0.05127] Death
  (`self.DisableInput` null)
  (`PrimitiveComponent.SetCollisionEnabled` _mesh "PhysicsOnly")
  (`PrimitiveComponent.SetCollisionResponseToChannel` _mesh "ECC_Pawn" "ECR_Block")
  (`PrimitiveComponent.SetSimulatePhysics` _mesh true)
  (`PrimitiveComponent.SetCollisionEnabled` (`self.Assassination Radius`) "NoCollision")
  (`ActorComponent.K2_DestroyComponent` (`self.CapsuleComponent`))
  (`SceneComponent.SetVisibility` (`self.Heath Bar Widget`) false false))

(event `Assassination Death`
  ;[0.05127 0.05127 0.05127] Assassination Death
  (`|ExecutionSequence`
    (:`then_0`
      (`PrimitiveComponent.SetCollisionEnabled` (`self.Mesh`) "PhysicsOnly")
      (`KismetSystemLibrary.Delay` 2.5)
      (`self.Die`))
    (:`then_1`
      (`KismetSystemLibrary.Delay` 1.7)
      (`GameplayStatics.PlaySoundAtLocation` "/Game/Audio/Grunts-Hits/SC_Death.SC_Death" (`self.K2_GetActorLocation`) (struct) 1.0 1.0 0.0 null null null null))))

(fn `Stealth Back Assassin`
  (returns (`REF Location` :type "Vector Structure") (`Assassin Rotation` :type "Rotator Structure"))
  (`PrimitiveComponent.SetCollisionEnabled` (`self.CapsuleComponent`) "NoCollision")
  (`self.PlayAnimMontage` "/Game/Characters/Base_Character/Animations/Assassination/Paired_Knife_Stealth_KidneyAndNeck_Vic_Montage.Paired_Knife_Stealth_KidneyAndNeck_Vic_Montage")
  (`self.Assassination Death`)
  (`SceneComponent.SetVisibility` (`self.Assassinate Widget`) false false)
  (return (`SceneComponent.K2_GetComponentLocation` (`self.Assassin REF`)) (`self.K2_GetActorRotation`)))

(fn `Update Health HUD`
  (bind _bpc_character_stats (`self.BPC_Character_Stats`))
  (bind _current_health (`/Game/Blueprints/BPC_Character_Stats.Current Health` _bpc_character_stats))
  (bind _max_health (`/Game/Blueprints/BPC_Character_Stats.Max Health` _bpc_character_stats))
  (`ProgressBar.SetPercent` (`/Game/UI/WB_DummyHealthBar.HealthBar` (`self.Health Bar Widget`)) (/ _current_health _max_health))
  (`TextBlock.SetText` (`/Game/UI/WB_DummyHealthBar.HealthText` (`self.Health Bar Widget`)) (`KismetTextLibrary.Conv_StringToText` (`KismetStringLibrary.Concat_StrStr` (`KismetStringLibrary.Concat_StrStr` (`KismetStringLibrary.Conv_DoubleToString` _current_health) "/") (`KismetStringLibrary.Conv_DoubleToString` _max_health)))))

(fn `Update HUD`
  (`self.Update Health HUD`))

(fn `UserConstructionScript`)