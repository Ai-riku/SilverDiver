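; Character stats component that tracks health, stamina, XP and level.
; Increase functions cap health and stamina at their maximums, while decrease functions floor them at zero and return whether the stat is depleted.
; Reaching the XP threshold carries over the surplus and raises the level, which plays a sound and grows the next threshold in proportion to level.
; Level-up calls itself recursively to resolve multiple levels from one XP gain.
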(event `self.ReceiveBeginPlay`)

(fn `Decrease Health`
  (params (`Health Decrease` :type "Float (double-precision)"))
  (returns (`Is Player Dead?` :type Boolean))
  (if (not (<= (`self.Current Health`) 0.0))
    (set `self.Current Health` (- (`self.Current Health`) `Health Decrease`))
    (if (<= (`self.Current Health`) 0.0)
      (set `self.Current Health` 0.0)
      (else
        (return false))))
  (return true))

(fn `Decrease Stamina`
  (params (`Stamina Decrease` :type "Float (double-precision)"))
  (returns (`Stamina Depleted` :type Boolean))
  (if (not (<= (`self.Current Stamina`) 0.0))
    (set `self.Current Stamina` (- (`self.Current Stamina`) `Stamina Decrease`))
    (if (<= (`self.Current Stamina`) 0.0)
      (set `self.Current Stamina` 0.0)
      (else
        (return false))))
  (return true))

(fn `Increase Health`
  (params (`Health Increase` :type "Float (double-precision)"))
  (bind _max_health (`self.Max Health`))
  (set `self.Current Health` (+ (`self.Current Health`) `Health Increase`))
  (if (> (`self.Current Health`) _max_health)
    (set `self.Current Health` _max_health)))

(fn `Increase Level`
  (params (`Level Increase` :type Integer))
  (set `self.Level` (+ (`self.Level`) `Level Increase`))
  (set `self.Max XP` (+ (`self.Max XP`) (* (`self.Level`) 50)))
  (`GameplayStatics.PlaySound2D` "/Game/Audio/UI/LevelUp1.LevelUp1" 1.0 1.0 0.0 null null)
  (if (>= (`self.XP`) (`self.Max XP`))
    (set `self.XP` (- (`self.XP`) (`self.Max XP`)))
    (`self.Increase Level` 1)))

(fn `Increase Max Health`
  (params (`Max Health Increase` :type "Float (double-precision)"))
  (set `self.Max Health` (+ (`self.Max Health`) `Max Health Increase`)))

(fn `Increase Max Stamina`
  (params (`Max Stamina Increase` :type "Float (double-precision)"))
  (set `self.Max Stamina` (+ (`self.Max Stamina`) `Max Stamina Increase`)))

(fn `Increase Stamina`
  (params (`Stamina Increase` :type "Float (double-precision)"))
  (bind _max_stamina (`self.Max Stamina`))
  (set `self.Current Stamina` (+ (`self.Current Stamina`) `Stamina Increase`))
  (if (> (`self.Current Stamina`) _max_stamina)
    (set `self.Current Stamina` _max_stamina)))

(fn `Increase XP`
  (params (`XP Increase` :type "Float (double-precision)"))
  (set `self.XP` (+ (`self.XP`) `XP Increase`))
  (if (>= (`self.XP`) (`self.Max XP`))
    (set `self.XP` (- (`self.XP`) (`self.Max XP`)))
    (`self.Increase Level` 1)))