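; Melee attack component for BP_ThirdPersonCharacter that handles combo montages, hit detection and damage.
; Attack input starts or buffers the next combo montage, which SwordAttackCombo continues or ends.
; Timer-driven traces sweep segments along the blade between previous and current samples, or follow the right foot for point attacks.
; DamageActor hits each "Damageable" actor once until tracing stops, adding camera shake, blood and sound.
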(event Custom|Play%20Sword%20Hit%20Sounds
  ;[0.05127 0.05127 0.05127] Play Sword Hit Sound
  (Audio|PlaySoundatLocation "/Game/Audio/Sword/MS_SwordHits.MS_SwordHits" (Transformation|GetActorLocation (Components|GetOwner)) "0, 0, 0" 1.0 1.0 0.0 0 0 0 0))

(event Custom|Sword%20Attack%20Combo
  ;[0.05127 0.05127 0.05127] Combo System
  ;;[0.05127 0.05127 0.05127] Combo Continue
  (if (Variables|ComboSystem|GetSave%20Attack?)
    (Variables|ComboSystem|SetSave%20Attack? false)
    ;;[0.05127 0.05127 0.05127] Attack Input
    (CallFunction|Attack)
    (else
      (CallFunction|StopCombo))))

(event Custom|Stop%20Sword%20Trace
  ;[0.05127 0.05127 0.05127] Sword Trace
  (Utilities|Time|ClearandInvalidateTimerbyHandle (Variables|Trace|GetTrace%20Timer))
  (Utilities|Set|Clear (Variables|Trace|GetDamaged%20Actors))
  (Utilities|Array|Clear (Variables|Trace|GetCurrent%20Sword%20Trace%20Segments))
  (Utilities|Array|Clear (Variables|Trace|GetPrevious%20Sword%20Trace%20Segments)))

(event Custom|Stop%20Combo
  ;[0.05127 0.05127 0.05127] Combo System
  ;;[0.05127 0.05127 0.05127] Stop Combo/Attack
  (Variables|ComboSystem|SetIs%20Attacking false)
  (Variables|ComboSystem|SetAttack%20Index 0))

(event Custom|Sword%20Trace%20Loop
  (bind _bp_character (Variables|Components|GetBP%20Character))
  (bind _sword_tip_point (Variables|/Game/ThirdPerson/Blueprints/BP_ThirdPersonCharacter.BP_ThirdPersonCharacter_C|GetSword%20Tip%20Point _bp_character))
  (bind _sword_base_point (Variables|/Game/ThirdPerson/Blueprints/BP_ThirdPersonCharacter.BP_ThirdPersonCharacter_C|GetSword%20Base%20Point _bp_character))
  (bind _returnvalue (Transformation|GetWorldLocation _sword_tip_point))
  (bind _returnvalue_2 (Transformation|GetWorldLocation _sword_base_point))
  ;[0.05127 0.05127 0.05127] Sword Trace
  (Collision|SphereTraceByChannel _returnvalue _returnvalue_2 0.0 "TraceTypeQuery1" false 0 (Variables|Default|GetDraw%20Debug%20Type) true "(R=1.000000,G=0.000000,B=0.000000,A=1.000000)" "(R=0.000000,G=1.000000,B=0.000000,A=1.000000)" 0.01)
  (for _index (range 0 5)
    (Utilities|Array|Add (Variables|Trace|GetCurrent%20Sword%20Trace%20Segments) (- _returnvalue (* (/ (- _returnvalue _returnvalue_2) 5.0) _index))))
  (if (> (Utilities|Array|Length (Variables|Trace|GetPrevious%20Sword%20Trace%20Segments)) 0)
    (for (_array_element _array_index) (Variables|Trace|GetPrevious%20Sword%20Trace%20Segments)
      (bind (_outhit _returnvalue_3) (Collision|SphereTraceByChannel _array_element (Utilities|Array|Get(acopy) (Variables|Trace|GetCurrent%20Sword%20Trace%20Segments) _array_index) 0.0 "TraceTypeQuery1" false 0 (Variables|Default|GetDraw%20Debug%20Type) true "(R=0.000000,G=0.137825,B=1.000000,A=1.000000)" "(R=0.000000,G=1.000000,B=0.000000,A=1.000000)" 0.1))
      (CallFunction|DamageActor _outhit _returnvalue_3))
    (Variables|Trace|SetPrevious%20Sword%20Trace%20Segments (Variables|Trace|GetCurrent%20Sword%20Trace%20Segments))
    (else
      (Variables|Trace|SetPrevious%20Sword%20Trace%20Segments (Variables|Trace|GetCurrent%20Sword%20Trace%20Segments))))
  (Utilities|Array|Clear (Variables|Trace|GetCurrent%20Sword%20Trace%20Segments)))

(event Custom|Start%20Point%20Damage%20Trace
  ;[0.05127 0.05127 0.05127] Point Damage Trace
  (bind _returnvalue (Utilities|Time|SetTimerbyEvent (delegate Custom|Point%20Damage%20Trace) 0.01 true))
  (Variables|Trace|SetTrace%20Timer _returnvalue))

(event Custom|Stop%20Point%20Damage%20Trace
  ;[0.05127 0.05127 0.05127] Point Damage Trace
  (Utilities|Time|ClearandInvalidateTimerbyHandle (Variables|Trace|GetTrace%20Timer))
  (Utilities|Set|Clear (Variables|Trace|GetDamaged%20Actors))
  (Variables|Trace|SetPrevious%20Point%20Trace "0, 0, 0"))

(event Custom|Point%20Damage%20Trace
  (bind _bp_character (Variables|Components|GetBP%20Character))
  (bind _right_foot (Variables|/Game/ThirdPerson/Blueprints/BP_ThirdPersonCharacter.BP_ThirdPersonCharacter_C|GetRight%20Foot _bp_character))
  (bind _returnvalue (Transformation|GetWorldLocation _right_foot))
  ;[0.05127 0.05127 0.05127] Point Damage Trace
  (if (not (Utilities|Operators|EqualEqual :A (Variables|Trace|GetPrevious%20Point%20Trace)))
    (bind (_outhit _returnvalue_2) (Collision|SphereTraceByChannel (stale _output_get) _returnvalue 12.0 "TraceTypeQuery1" false 0 (Variables|Default|GetDraw%20Debug%20Type) true "(R=1.000000,G=0.000000,B=0.000000,A=1.000000)" "(R=0.000000,G=1.000000,B=0.000000,A=1.000000)" 0.01))
    (CallFunction|DamageActor _outhit _returnvalue_2)
    (Variables|Trace|SetPrevious%20Point%20Trace "0, 0, 0")
    (else
      (bind _output_get (Variables|Trace|SetPrevious%20Point%20Trace _returnvalue)))))

(event Custom|Attack
  (bind _attack_combo (Variables|ComboSystem|GetAttack%20Combo))
  ;[0.05127 0.05127 0.05127] Combo System
  ;;[0.05127 0.05127 0.05127] Attack
  (Utilities|FlowControl|DoOnce false :!label _label
    (:Completed
      (Animation|Montage|PlayMontage (Variables|Default|GetCharacter%20Mesh) (Utilities|Array|Get(acopy) _attack_combo (Variables|ComboSystem|GetAttack%20Index))
        (:then
          (if (< (Variables|ComboSystem|GetAttack%20Index) (Utilities|Array|Length _attack_combo))
            (Variables|ComboSystem|SetAttack%20Index (+ (Variables|ComboSystem|GetAttack%20Index) 1))
            (goto _label Reset)
            (else
              (Variables|ComboSystem|SetAttack%20Index 0)
              (goto _label Reset))))))))

(event Custom|Start%20Sword%20Trace
  ;[0.05127 0.05127 0.05127] Sword Trace
  (bind _returnvalue (Utilities|Time|SetTimerbyEvent (delegate Custom|Sword%20Trace%20Loop) 0.01 true))
  (Variables|Trace|SetTrace%20Timer _returnvalue))

(event Input|EnhancedActionEvents|EnhancedInputActionIA_Attack
  (params (ActionValue :type Boolean) (ElapsedSeconds :type Float%20%28double-precision%29) (TriggeredSeconds :type Float%20%28double-precision%29) (InputAction :type Input%20Action%20Object%20Reference :default "/Game/ThirdPerson/Input/Actions/IA_Attack.IA_Attack"))
  ;[0.05127 0.05127 0.05127] Combo System
  ;;[0.05127 0.05127 0.05127] Attack Input
  (:Started
    (if (Variables|ComboSystem|GetCan%20Attack)
      (if (Variables|ComboSystem|GetIs%20Attacking)
        (Variables|ComboSystem|SetSave%20Attack? true)
        (else
          (Variables|ComboSystem|SetIs%20Attacking true)
          (CallFunction|Attack))))))

(event EventBeginPlay
  (bind _asbp_third_person_character (Utilities|Casting|CastToBP_ThirdPersonCharacter (Components|GetOwner)))
  (Variables|Components|SetBP%20Character _asbp_third_person_character)
  (Variables|Default|SetCharacter%20Mesh (Variables|/Script/Engine.Character|GetMesh _asbp_third_person_character)))

(event EventTick
  (params (DeltaSeconds :type Float%20%28single-precision%29)))

(event Input|KeyboardEvents|DebugKeyDecimal
  (params (Key :type Key%20Structure :default "None") (ActionValue :type Input%20Action%20Value%20Structure))
  (:Pressed
    (bind _asbp_third_person_character (Utilities|Casting|CastToBP_ThirdPersonCharacter (Components|GetOwner)))
    (if (Variables|/Script/Engine.SceneComponent|GetbVisible (Variables|/Script/Engine.Character|GetMesh _asbp_third_person_character))
      (Rendering|SetVisibility (Variables|/Script/Engine.Character|GetMesh _asbp_third_person_character) false true)
      (else
        (Rendering|SetVisibility (Variables|/Script/Engine.Character|GetMesh _asbp_third_person_character) true true)))))

(event Input|KeyboardEvents|DebugKeyDivide
  (params (Key :type Key%20Structure :default "None") (ActionValue :type Input%20Action%20Value%20Structure))
  (bind _bp_character (Variables|Components|GetBP%20Character))
  (bind _followcamera (Variables|/Game/ThirdPerson/Blueprints/BP_ThirdPersonCharacter.BP_ThirdPersonCharacter_C|GetFollowCamera _bp_character))
  (bind _returnvalue (Transformation|GetWorldLocation _followcamera))
  (:Pressed
    (Collision|LineTraceByChannel _returnvalue (+ _returnvalue (* (Math|Vector|GetForwardVector (Transformation|GetWorldRotation _followcamera)) 2e+03)) "TraceTypeQuery1" false 0 "ForDuration")))

(fn DamageActor
  (params (Hit :type Hit%20Result%20Structure%20%28by%20ref%29) (Condition :type Boolean))
  (bind (_bblockinghit _binitialoverlap _time _distance _location _impactpoint _normal _impactnormal _physmat _hitactor) (Collision|BreakHitResult Hit))
  (if Condition
    (if (Actor|ActorHasTag _hitactor "Damageable")
      (if (not (Utilities|Set|Contains (Variables|Trace|GetDamaged%20Actors) _hitactor))
        (Utilities|Set|Add (Variables|Trace|GetDamaged%20Actors) _hitactor)
        (Game|Damage|ApplyDamage _hitactor 25.0 0 0)
        (Camera|PlayWorldCameraShake "/Game/Blueprints/BP_Sword_Hit_CameraShake.BP_Sword_Hit_CameraShake_C" _location 0.0 2e+03)
        (Effects|SpawnEmitteratLocation "/Game/VFX/Particles/Blood/P_Blood_Splat_Cone.P_Blood_Splat_Cone" _location (Math|Rotator|MakeRotfromZ _normal) "0.400000,0.400000,0.400000" true "AutoRelease")
        (Effects|SpawnEmitteratLocation "/Game/VFX/Particles/Blood/P_Blood_Splat_Cone.P_Blood_Splat_Cone" _location (Math|Rotator|MakeRotfromZ (* _normal -1.0)) "0.200000,0.200000,0.200000" true "AutoRelease")
        (CallFunction|PlaySwordHitSounds)))))